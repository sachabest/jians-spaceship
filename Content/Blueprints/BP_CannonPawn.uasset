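; Player-controlled cannon pawn that attaches itself to the Arrow component of the first BPI_Ship actor, expected to be a BP_ShipPawn.
; F toggles whether the ShipYaw and ShipPitch axes aim the cannon or rotate only the camera.
; Remote instances apply aim locally and forward it through Server events, while authority applies it directly.
; Cannon pitch is limited between -20 and 80 degrees, and pitching recentres the camera.
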(event `self.ReceiveBeginPlay`
  (bind _outactors (`GameplayStatics.GetAllActorsWithInterface` "/Game/Blueprints/BPI_Ship.BPI_Ship_C"))
  (bind _asbp_ship_pawn (cast `/Game/Blueprints/BP_ShipPawn` (`KismetArrayLibrary.Array_Get` _outactors)))
  (`self.K2_AttachRootComponentTo` (`/Game/Blueprints/BP_ShipPawn.Arrow` _asbp_ship_pawn) "None" "SnapToTarget"))

(event `CannonYaw`
  (params (AxisValue :type "Float (double-precision)"))
  ;[1 1 1] Yaw
  (`SceneComponent.K2_AddWorldRotation` (`self.Root`) (`KismetMathLibrary.MakeRotator` 0.0 0.0 (* AxisValue 2.0)) false false))

(event `InputAxis|ShipYaw`
  (params (AxisValue :type "Float (single-precision)"))
  ;[1 1 1] Yaw
  (if (`self.IsControlling`)
    (`/Engine/EditorBlueprintResources/ActorMacros.Switch Has Authority`
      (:`Authority`
        (`self.CannonYaw` AxisValue))
      (:`Remote`
        (`self.ServerYaw` AxisValue)
        (`self.CannonYaw` AxisValue)))
    (else
      (`SceneComponent.K2_AddLocalRotation` (`self.Camera`) (`KismetMathLibrary.MakeRotator` 0.0 0.0 (* AxisValue 2.0)) false false))))

(event `ServerYaw`
  (params (AxisValue :type "Float (double-precision)"))
  ;[1 1 1] Yaw
  (`self.CannonYaw` AxisValue))

(event `Key|F`
  (params (Key :type "Key Structure" :default "LeapLeftPinch"))
  (:`Pressed`
    (set `self.IsControlling` (not (`self.IsControlling`)))))

(event `InputAxis|ShipPitch`
  (params (AxisValue :type "Float (single-precision)"))
  ;[1 1 1] Pitch
  (if (`self.IsControlling`)
    (`/Engine/EditorBlueprintResources/ActorMacros.Switch Has Authority`
      (:`Authority`
        (`self.CannonPitch` AxisValue))
      (:`Remote`
        (`self.ServerPitch` AxisValue)
        (`self.CannonPitch` AxisValue)))
    (else
      (`SceneComponent.K2_AddLocalRotation` (`self.Camera`) (`KismetMathLibrary.MakeRotator` 0.0 (* AxisValue -2.0)) false false))))

(event `CannonPitch`
  (params (AxisValue :type "Float (double-precision)"))
  (bind _pitch (.pitch (`SceneComponent.K2_GetComponentRotation` (`self.Root`))))
  ;[1 1 1] Pitch
  (if (not (or (and (> _pitch 80.0) (< AxisValue 0.0)) (and (< _pitch -20.0) (> AxisValue 0.0))))
    (`SceneComponent.K2_AddLocalRotation` (`self.Root`) (`KismetMathLibrary.MakeRotator` 0.0 (* AxisValue -2.0)) false false)
    (`SceneComponent.K2_SetRelativeRotation` :`self` (`self.Camera`))))

(event `ServerPitch`
  (params (AxisValue :type "Float (double-precision)"))
  ;[1 1 1] Pitch
  (`self.CannonPitch` AxisValue))

(fn `UserConstructionScript`)