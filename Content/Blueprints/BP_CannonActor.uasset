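; BP_CannonActor is a turret weapon that rotates and fires BP_FriendlyProjectile from its barrel.
; Pitch and yaw events add relative rotation to separate gun components, blocking further movement beyond fixed angular limits in each direction.
; FireProjectile and ServerFireProjectile run identical logic, spawning the projectile at the GunBarrelDirection transform with the passed-in owner.
; The logic that attaches it to BP_CannonPawn is disconnected, so BeginPlay does nothing.
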(event `ChangeTurretPitch`
  (params (DeltaYawDegrees :type "Float (double-precision)"))
  (bind _gunpitchcomponent (`self.GunPitchComponent`))
  (bind (_relativerotation_roll _relativerotation_pitch) (`KismetMathLibrary.BreakRotator` (`SceneComponent.RelativeRotation` _gunpitchcomponent)))
  ;[1 1 1] Turret Pitch / Vertical Rotation
  (if (or (and (>= _relativerotation_pitch -60.0) (< DeltaYawDegrees 0.0)) (and (<= _relativerotation_pitch 60.0) (> DeltaYawDegrees 0.0)))
    (`SceneComponent.K2_AddRelativeRotation` _gunpitchcomponent (`KismetMathLibrary.MakeRotator` 0.0 DeltaYawDegrees) false false)))

(event `ChangeTurretYaw`
  (params (DeltaYawDegrees :type "Float (double-precision)"))
  (bind _gunyawcomponent (`self.GunYawComponent`))
  (bind (_relativerotation_roll _relativerotation_pitch _relativerotation_yaw) (`KismetMathLibrary.BreakRotator` (`SceneComponent.RelativeRotation` _gunyawcomponent)))
  ;[1 1 1] Turret Yaw / Horizontal Rotation
  (if (or (and (>= _relativerotation_yaw -80.0) (< DeltaYawDegrees 0.0)) (and (<= _relativerotation_yaw 80.0) (> DeltaYawDegrees 0.0)))
    (`SceneComponent.K2_AddRelativeRotation` _gunyawcomponent (`KismetMathLibrary.MakeRotator` 0.0 0.0 DeltaYawDegrees) false false)))

(event `ServerFireProjectile`
  (params (Owner :type "PlayerController Object Reference"))
  (bind (_returnvalue_location _returnvalue_rotation) (`KismetMathLibrary.BreakTransform` (`SceneComponent.K2_GetComponentToWorld` (`self.GunBarrelDirection`))))
  ;[1 1 1] Fires a laser from the gun barrel
  (bind _asactor (castclass `Actor` (`KismetMathLibrary.SelectClass` "/Game/Blueprints/BP_FriendlyProjectile.BP_FriendlyProjectile_C" null true)))
  (`|SpawnActorFromClass` _asactor (`KismetMathLibrary.MakeTransform` _returnvalue_location _returnvalue_rotation) "Undefined" "OverrideRootScale" Owner))

(event `FireProjectile`
  (params (Owner :type "PlayerController Object Reference"))
  (bind (_returnvalue_location _returnvalue_rotation) (`KismetMathLibrary.BreakTransform` (`SceneComponent.K2_GetComponentToWorld` (`self.GunBarrelDirection`))))
  ;[1 1 1] Fires a laser from the gun barrel
  (bind _asactor (castclass `Actor` (`KismetMathLibrary.SelectClass` "/Game/Blueprints/BP_FriendlyProjectile.BP_FriendlyProjectile_C" null true)))
  (`|SpawnActorFromClass` _asactor (`KismetMathLibrary.MakeTransform` _returnvalue_location _returnvalue_rotation) "Undefined" "OverrideRootScale" Owner))

(event `self.ReceiveBeginPlay`
  ;[1 1 1] Attach this weapon to the gunner
)

(fn `UserConstructionScript`)