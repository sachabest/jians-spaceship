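; BP_BPSwitch is a switch-type breaking point that is resolved when a qualifying component overlaps its Box trigger.
; It extends the parent's Break and Resolve events by swapping the Cube's material to Off when broken and On when resolved or constructed.
; An overlap calls Resolve only if IsGoodCollision accepts the component and ActiveTimerHandle is still valid.
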(event `self.Break`
  (`parent.Break`)
  (`PrimitiveComponent.SetMaterial` (`self.Cube`) 0 (`|ConvertAsset` (`self.Off`))))

(event `self.Resolve`
  (`parent.Resolve`)
  (`PrimitiveComponent.SetMaterial` (`self.Cube`) 0 (`|ConvertAsset` (`self.On`))))

(event `self.Box.OnComponentBeginOverlap`
  (params (OtherActor :type "Actor Object Reference") (OtherComp :type "PrimitiveComponent Object Reference") (OtherBodyIndex :type Integer) (bFromSweep :type Boolean) (SweepResult :type "HitResult Structure (by ref)"))
  (bind _good (`self.IsGoodCollision` OtherComp))
  (if (and _good (`KismetSystemLibrary.K2_IsValidTimerHandle` (`self.ActiveTimerHandle`)))
    (`self.Resolve`)))

(fn `UserConstructionScript`
  (`parent.UserConstructionScript`)
  (`PrimitiveComponent.SetMaterial` (`self.Cube`) 0 (`|ConvertAsset` (`self.On`))))