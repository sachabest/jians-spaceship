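; BP_BPLever is a breaking-point lever that can be broken and then repaired by a valid overlap.
; It extends parent Break and Resolve events, tracking an IsBroken flag alongside them.
; An overlap on its capsule that passes IsGoodCollision resolves it while broken.
; Tick smoothly interpolates the lever's pitch between two opposite angles according to the broken state.
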(event `self.Resolve`
  (`parent.Resolve`)
  (set `self.IsBroken` false))

(event `self.Break`
  (`parent.Break`)
  (set `self.IsBroken` true))

(event `self.Capsule.OnComponentBeginOverlap`
  (params (OtherActor :type "Actor Object Reference") (OtherComp :type "PrimitiveComponent Object Reference") (OtherBodyIndex :type Integer) (bFromSweep :type Boolean) (SweepResult :type "HitResult Structure (by ref)"))
  (bind _good (`self.IsGoodCollision` OtherComp))
  (if (and _good (`self.IsBroken`))
    (`self.Resolve`)))

(event `self.ReceiveTick`
  (params (DeltaSeconds :type "Float (single-precision)"))
  (bind _leverrotation (`self.LeverRotation`))
  (bind _relativerotation (`SceneComponent.RelativeRotation` _leverrotation))
  (if (`self.IsBroken`)
    (`SceneComponent.K2_SetRelativeRotation` _leverrotation (`KismetMathLibrary.RInterpTo` _relativerotation (struct :`Roll` 50.0) DeltaSeconds 6.0) false false)
    (else
      (`SceneComponent.K2_SetRelativeRotation` _leverrotation (`KismetMathLibrary.RInterpTo` _relativerotation (struct :`Roll` -50.0) DeltaSeconds 6.0) false false))))

(fn `UserConstructionScript`
  (`parent.UserConstructionScript`))