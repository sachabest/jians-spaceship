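; BP_BreakingPoint is a timed breaking point that reports a failure to the game mode if it is not resolved before its timeout.
; Break starts a one-shot timer, Resolve clears it, and expiry calls BreakingPointFailed on MyGameMode.
; Helper functions match a component's object name against the Colliders list, either validating the collision or returning its index as the hand, with -1 for no match.
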(event `Break`
  (bind _returnvalue (`KismetSystemLibrary.K2_SetTimerDelegate` (delegate `Fail`) (`self.Timeout`)))
  (set `self.ActiveTimerHandle` _returnvalue))

(event `Resolve`
  (`KismetSystemLibrary.K2_ClearTimerHandle` (`self.ActiveTimerHandle`))
  (set `self.ActiveTimerHandle` (struct) :!label _label))

(event `Fail`
  (bind _asmy_game_mode (cast `/Game/Blueprints/MultiPlayer/MyGameMode` (`GameplayStatics.GetGameMode`)))
  (`/Game/Blueprints/MultiPlayer/MyGameMode.BreakingPointFailed` _asmy_game_mode)
  (goto _label))

(fn `IsGoodCollision`
  (params (Component :type "ActorComponent Object Reference"))
  (returns (Good :type Boolean))
  (return (`KismetArrayLibrary.Array_Contains` (`self.Colliders`) (`KismetSystemLibrary.GetObjectName` Component))))

(fn `UserConstructionScript`)

(fn `WhichHand`
  (params (Component :type "PrimitiveComponent Object Reference"))
  (returns (Which :type Integer))
  (for (_array_element _array_index) (`self.Colliders`)
    (if (`KismetStringLibrary.EqualEqual_StrStr` _array_element (`KismetSystemLibrary.GetObjectName` Component))
      (return _array_index)))
  (return -1))