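; Player-flown ship pawn with thrust, yaw and pitch axis controls and a count of gates flown through.
; F toggles control between steering the ship and rotating only the camera; ship yaw resets the camera's relative rotation.
; Ship inputs apply locally, with non-authority instances also calling Server events that repeat the movement.
; ShipFlewThroughGate increments and prints the gate count, while both getter functions return only zero values.
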(event `self.ReceiveBeginPlay`
  (set `self.ControllerRef` (`GameplayStatics.GetPlayerController` 0)))

(event `/Game/Blueprints/BPI_Ship.shipFlewThroughGate`
  (bind _output_get (set `self.GateFlownThrough` (+ (`self.GateFlownThrough`) 1)))
  (`KismetSystemLibrary.PrintString` (`KismetStringLibrary.Concat_StrStr` "Number of Gates:" (`KismetStringLibrary.Conv_IntToString` _output_get))))

(event `ShipThrust`
  (params (AxisValue :type "Float (double-precision)"))
  ;[1 1 1] Thrust
  (`self.AddMovementInput` (* (`SceneComponent.GetForwardVector` (`self.Root`)) (* AxisValue 5.0))))

(event `ServerThrust`
  (params (AxisValue :type "Float (double-precision)"))
  ;[1 1 1] Thrust
  (`self.ShipThrust` AxisValue))

(event `InputAxis|MainThrust`
  (params (AxisValue :type "Float (single-precision)"))
  ;[1 1 1] Thrust
  (if (`self.IsControlling`)
    (`/Engine/EditorBlueprintResources/ActorMacros.Switch Has Authority`
      (:`Authority`
        _)
      (:`Remote`
        (`self.ServerThrust` AxisValue)))
    (`self.ShipThrust` AxisValue)))

(event `ShipYaw`
  (params (AxisValue :type "Float (double-precision)"))
  ;[1 1 1] ShipYaw
  (`SceneComponent.K2_AddWorldRotation` (`self.Root`) (`KismetMathLibrary.MakeRotator` 0.0 0.0 (* AxisValue 2.0)) false false)
  (`SceneComponent.K2_SetRelativeRotation` :`self` (`self.Camera`)))

(event `ServerYaw`
  (params (AxisValue :type "Float (double-precision)"))
  ;[1 1 1] ShipYaw
  (`self.ShipYaw` AxisValue))

(event `InputAxis|ShipYaw`
  (params (AxisValue :type "Float (single-precision)"))
  ;[1 1 1] ShipYaw
  (if (`self.IsControlling`)
    (`/Engine/EditorBlueprintResources/ActorMacros.Switch Has Authority`
      (:`Authority`
        _)
      (:`Remote`
        (`self.ServerYaw` AxisValue)))
    (`self.ShipYaw` AxisValue)
    (else
      (`SceneComponent.K2_AddLocalRotation` (`self.Camera`) (`KismetMathLibrary.MakeRotator` 0.0 0.0 (* AxisValue 2.0)) false false))))

(event `ShipPitch`
  (params (AxisValue :type "Float (double-precision)"))
  ;[1 1 1] ShipPitch
  (`SceneComponent.K2_AddLocalRotation` (`self.Root`) (`KismetMathLibrary.MakeRotator` 0.0 (* AxisValue -2.0)) false false))

(event `ServerPitch`
  (params (AxisValue :type "Float (double-precision)"))
  ;[1 1 1] ShipPitch
  (`self.ShipPitch` AxisValue))

(event `InputAxis|ShipPitch`
  (params (AxisValue :type "Float (single-precision)"))
  ;[1 1 1] ShipPitch
  (if (`self.IsControlling`)
    (`/Engine/EditorBlueprintResources/ActorMacros.Switch Has Authority`
      (:`Authority`
        _)
      (:`Remote`
        (`self.ServerPitch` AxisValue)))
    (`self.ShipPitch` AxisValue)
    (else
      (`SceneComponent.K2_AddLocalRotation` (`self.Camera`) (`KismetMathLibrary.MakeRotator` 0.0 (* AxisValue -2.0)) false false))))

(event `Key|F`
  (params (Key :type "Key Structure" :default "LeapLeftPinch"))
  (:`Pressed`
    (set `self.IsControlling` (not (`self.IsControlling`)))))

(fn `getNumGatesFlownThrough`
  (returns (Num :type Integer))
  (return 0))

(fn `getShipRotation`
  (returns (ShipRotation :type "Rotator Structure"))
  (return))

(fn `UserConstructionScript`)