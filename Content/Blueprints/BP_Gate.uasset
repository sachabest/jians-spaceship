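; BP_Gate is a server-authoritative, timed gate that rewards a ship flying through it with cannon ammunition.
; On BeginPlay it starts a lifetime timer and polls until it finds the BP_CannonPawn.
; The first ship to exit its box cancels expiry, gets notified, and after a delay the gate leaves MyGameMode's Gates list and adds ammunition.
; Only expiry, not a fly-through, calls ReseedGates when the list empties.
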(event `FindCannonPawn`
  (bind _outactors (`GameplayStatics.GetAllActorsOfClass` "/Game/Blueprints/BP_CannonPawn.BP_CannonPawn_C"))
  (if (not (== (`KismetArrayLibrary.Array_Length` _outactors) 0))
    (set `self.CannonPawnRef` (`KismetArrayLibrary.Array_Get` _outactors))
    (`KismetSystemLibrary.K2_ClearTimerHandle` (`self.FindCannonPawnTimer`))))

(event `self.ReceiveBeginPlay`
  (`/Engine/EditorBlueprintResources/ActorMacros.Switch Has Authority`
    (:`Authority`
      (bind _returnvalue (`KismetSystemLibrary.K2_SetTimerDelegate` (delegate `DestroyGate`) (`self.LifeTime`)))
      (set `self.RespawnTimer` _returnvalue)
      (bind _returnvalue_2 (`KismetSystemLibrary.K2_SetTimerDelegate` (delegate `FindCannonPawn`) 0.5 true))
      (set `self.FindCannonPawnTimer` _returnvalue_2))))

(event `DestroyGate`
  (`self.K2_DestroyActor`)
  (bind _asmy_game_mode (cast `/Game/Blueprints/MultiPlayer/MyGameMode` (`GameplayStatics.GetGameMode`)))
  (bind _gates (`/Game/Blueprints/MultiPlayer/MyGameMode.Gates` _asmy_game_mode))
  (`KismetArrayLibrary.Array_RemoveItem` _gates self)
  (if (== (`KismetArrayLibrary.Array_Length` _gates) 0)
    (bind _asmy_game_mode_2 (cast `/Game/Blueprints/MultiPlayer/MyGameMode` (`GameplayStatics.GetGameMode`)))
    (`/Game/Blueprints/MultiPlayer/MyGameMode.ReseedGates` _asmy_game_mode_2)))

(event `self.Box Collision.OnComponentEndOverlap`
  (params (OtherActor :type "Actor Object Reference") (OtherComp :type "PrimitiveComponent Object Reference") (OtherBodyIndex :type Integer))
  (bind _cannonpawnref (`self.CannonPawnRef`))
  (`/Engine/EditorBlueprintResources/ActorMacros.Switch Has Authority`
    (:`Authority`
      (bind _asbp_ship_pawn (cast `/Game/Blueprints/BP_ShipPawn` OtherActor))
      (`/Engine/EditorBlueprintResources/StandardMacros.DoOnce` false
        (:`Completed`
          (`KismetSystemLibrary.K2_ClearTimerHandle` (`self.RespawnTimer`))
          (message `/Game/Blueprints/BPI_Ship.shipFlewThroughGate` _asbp_ship_pawn)
          (`KismetSystemLibrary.Delay` 1.0)
          (`self.K2_DestroyActor`)
          (bind _asmy_game_mode (cast `/Game/Blueprints/MultiPlayer/MyGameMode` (`GameplayStatics.GetGameMode`)))
          (`KismetArrayLibrary.Array_RemoveItem` (`/Game/Blueprints/MultiPlayer/MyGameMode.Gates` _asmy_game_mode) self)
          (set `/Game/Blueprints/BP_CannonPawn.Ammunition` (+ (`/Game/Blueprints/BP_CannonPawn.Ammunition` _cannonpawnref) 20.0) _cannonpawnref))))))

(fn `UserConstructionScript`)